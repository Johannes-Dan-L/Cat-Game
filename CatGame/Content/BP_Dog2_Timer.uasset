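; Dog actor that makes its mesh appear and disappear on a fixed timed schedule.
; BeginPlay hides the mesh, reveals it after an initial wait, then runs a chain of Delays toggling visibility with short and long gaps.
; Each reveal reapplies the same material and enables query and physics collision, which is never disabled when hidden.
; A 20-count loop at the end feeds back into the Delay chain to repeat the cycle.
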(event `self.ReceiveBeginPlay`
  (`PrimitiveComponent.SetMaterial` (`self.Dog_Mesh`) 0 "/Game/2DSideScrollerBP/Dog/Dog_Mat.Dog_Mat")
  (`KismetSystemLibrary.Delay` 0.0)
  (`SceneComponent.SetVisibility` (`self.Dog_Mesh`) false false)
  (`KismetSystemLibrary.Delay` 8.0)
  (`PrimitiveComponent.SetMaterial` (`self.Dog_Mesh`) 0 "/Game/2DSideScrollerBP/Dog/Dog_Mat.Dog_Mat")
  (`SceneComponent.SetVisibility` (`self.Dog_Mesh`) true false)
  (`PrimitiveComponent.SetCollisionEnabled` (`self.Dog_Mesh`) "QueryAndPhysics")
  (`PrimitiveComponent.SetMaterial` (`self.Dog_Mesh`) 0 "/Game/2DSideScrollerBP/Dog/Dog_Mat.Dog_Mat" :!label _label)
  (`KismetSystemLibrary.Delay` 2.0)
  (`SceneComponent.SetVisibility` (`self.Dog_Mesh`) false false)
  (`KismetSystemLibrary.Delay` 2.0)
  (`PrimitiveComponent.SetMaterial` (`self.Dog_Mesh`) 0 "/Game/2DSideScrollerBP/Dog/Dog_Mat.Dog_Mat")
  (`SceneComponent.SetVisibility` (`self.Dog_Mesh`) true false)
  (`PrimitiveComponent.SetCollisionEnabled` (`self.Dog_Mesh`) "QueryAndPhysics")
  (`PrimitiveComponent.SetMaterial` (`self.Dog_Mesh`) 0 "/Game/2DSideScrollerBP/Dog/Dog_Mat.Dog_Mat")
  (`KismetSystemLibrary.Delay` 2.0)
  (`SceneComponent.SetVisibility` (`self.Dog_Mesh`) false false)
  (`KismetSystemLibrary.Delay` 14.0)
  (`PrimitiveComponent.SetMaterial` (`self.Dog_Mesh`) 0 "/Game/2DSideScrollerBP/Dog/Dog_Mat.Dog_Mat")
  (`SceneComponent.SetVisibility` (`self.Dog_Mesh`) true false)
  (`PrimitiveComponent.SetCollisionEnabled` (`self.Dog_Mesh`) "QueryAndPhysics")
  (for _ (range 1 21)
    (goto _label)))

(fn `UserConstructionScript`)