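; BP_Dog6_Timer is an actor that makes a dog mesh blink in and out of view on a fixed timer.
; From BeginPlay, chained delays show the mesh briefly, hide it for a much longer stretch, then restore its material, visibility and collision.
; The chain wires back into its own ForLoop, so it repeats through re-entry rather than the loop count.
; Collision is re-enabled each cycle but never disabled in this graph.
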(event `self.ReceiveBeginPlay`
  (for _ (range 1 21) :!label _label
    (`PrimitiveComponent.SetMaterial` (`self.Dog_Mesh`) 0 "/Game/2DSideScrollerBP/Dog/Dog_Mat.Dog_Mat")
    (`KismetSystemLibrary.Delay` 2.0)
    (`SceneComponent.SetVisibility` (`self.Dog_Mesh`) false false)
    (`KismetSystemLibrary.Delay` 18.0)
    (`PrimitiveComponent.SetMaterial` (`self.Dog_Mesh`) 0 "/Game/2DSideScrollerBP/Dog/Dog_Mat.Dog_Mat")
    (`SceneComponent.SetVisibility` (`self.Dog_Mesh`) true false)
    (`PrimitiveComponent.SetCollisionEnabled` (`self.Dog_Mesh`) "QueryAndPhysics")
    (goto _label)))

(fn `UserConstructionScript`)